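; BP_FPSBullet is a projectile actor that reacts when its sphere collider hits something.
; On hit it spawns an explosion particle once and pushes physics-simulating components with an impulse scaled from the bullet's velocity.
; If the hit actor is an enemy character, it calls that character's OnTakeDamage with a fixed force and the bullet's location.
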(event OnComponentHit(Sphere)
  (params (HitComponent :type Primitive%20Component%20Object%20Reference) (OtherActor :type Actor%20Object%20Reference) (OtherComp :type Primitive%20Component%20Object%20Reference) (NormalImpulse :type Vector :default "0, 0, 0") (Hit :type Hit%20Result%20Structure%20%28by%20ref%29))
  (bind _returnvalue (Transformation|GetActorLocation))
  (Utilities|FlowControl|Sequence
    (:then_0
      (Utilities|FlowControl|DoOnce false
        (:Completed
          (Effects|SpawnEmitteratLocation "/Game/InfimaGames/FreeFPSTemplate/Demo/VFX/Particles/P_Explosion.P_Explosion" (Transformation|GetActorLocation)))))
    (:then_1
      (if (Physics|IsSimulatingPhysics OtherComp "None")
        (Physics|AddImpulseatLocation OtherComp (* (Transformation|GetVelocity) "100.000000,100.000000,100.000000") _returnvalue "None")))
    (:then_2
      (bind _asbp_character_ennemi (Utilities|Casting|CastToBP_Character_Ennemi OtherActor))
      (Default|OnTakeDamage _asbp_character_ennemi "1.000000,1.000000,1.000000" _returnvalue))))

(event EventBeginPlay)

(event Collision|EventActorBeginOverlap
  (params (OtherActor :type Actor%20Object%20Reference)))

(event EventTick
  (params (DeltaSeconds :type Float%20%28single-precision%29)))

(fn ConstructionScript)