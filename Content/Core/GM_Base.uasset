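; Base game mode that runs enemy waves, score, HUD and adaptive music.
; BeginPlay starts calm music, triggers every BP_Spawner and creates the HUD; CheckWave respawns when no enemy AI controllers remain.
; AddScore applies a multiplier and schedules its reset, but also resets it immediately before incrementing.
; CheckMusic swaps calm and stress tracks using enemy and chaser counts, evaluated only while looping over chasing enemies.
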(event Custom|AddScore
  (Variables|Default|SetCurrentScore (+ (Variables|Default|GetCurrentScore) (* 1e+01 (Variables|Default|GetCurrentMultiplier))))
  (Utilities|Time|ClearandInvalidateTimerbyHandle (Variables|Default|GetTimerMultiplierHandle))
  (Utilities|Time|SetTimerbyFunctionName 0 "ResetMultiplier" 3.0)
  (CallFunction|ResetMultiplier)
  (if (< (Variables|Default|GetCurrentMultiplier) 5.0)
    (Variables|Default|SetCurrentMultiplier (+ (Variables|Default|GetCurrentMultiplier) 1.0))
    (Default|UpdateHUD (stale EventBeginPlay _output_get_2))))

(event Custom|ResetMultiplier
  (Variables|Default|SetCurrentMultiplier 1.0))

(event Custom|SpawnEnnemies
  (bind _outactors (Actor|GetAllActorsOfClass "/Game/ThirdPerson/Blueprints/BP_Spawner.BP_Spawner_C"))
  (for _array_element _outactors
    (bind _output_get (Variables|Default|SetSpawner _array_element))
    (bind _asbp_spawner (Utilities|Casting|CastToBP_Spawner _output_get))
    (Default|OnSpawnEnnemi _asbp_spawner)))

(event Custom|CheckWave
  (bind _outactors (Actor|GetAllActorsOfClass "/Game/ThirdPerson/Blueprints/AIC_Ennemi.AIC_Ennemi_C"))
  (if (== (Utilities|Array|Length _outactors) 0)
    (CallFunction|SpawnEnnemies)
    (elif true
      _)))

(event Custom|CheckMusic
  (Variables|Default|SetEnnemiesInChase 0.0)
  (bind _outactors (Actor|GetAllActorsOfClass "/Game/ThirdPerson/Blueprints/AIC_Ennemi.AIC_Ennemi_C"))
  (for _array_element _outactors
    (if (Variables|/Game/ThirdPerson/Blueprints/AIC_Ennemi.AIC_Ennemi_C|GetIsChasing _array_element)
      (Variables|Default|SetEnnemiesInChase (+ (Variables|Default|GetEnnemiesInChase) 1.0))
      (if (Math|Conversions|ToBoolean(Integer) (Class|KismetMathLibrary|OrIntInt (Math|Conversions|ToInteger(Boolean) (> (Utilities|Array|Length _outactors) 15)) (Math|Conversions|ToInteger(Boolean) (>= (Variables|Default|GetEnnemiesInChase) 5.0))))
        (if (not (Variables|Default|GetStressMusicPlaying))
          (Audio|Components|Audio|Stop (Variables|Default|GetCalmMusic))
          (bind _returnvalue (Audio|CreateSound2D "/Game/Sounds_BPs/MS_MusicStress_00.MS_MusicStress_00" 1.0 1.0 0.0 0))
          (bind _output_get (Variables|Default|SetStressMusic _returnvalue))
          (Audio|Components|Audio|Play _output_get 0.0)
          (Variables|Default|SetStressMusicPlaying true)
          (Variables|Default|SetCalmMusicPlaying false))
        (elif (Math|Conversions|ToBoolean(Integer) (Class|KismetMathLibrary|AndIntInt (Math|Conversions|ToInteger(Boolean) (< (Utilities|Array|Length _outactors) 5)) (Math|Conversions|ToInteger(Boolean) (<= (Variables|Default|GetEnnemiesInChase) 2.0))))
          (if (not (Variables|Default|GetCalmMusicPlaying))
            (Audio|Components|Audio|Stop (Variables|Default|GetStressMusic))
            (bind _returnvalue_2 (Audio|CreateSound2D "/Game/Sounds_BPs/MS_MusicCalm_00.MS_MusicCalm_00" 1.0 1.0 0.0 0))
            (bind _output_get_2 (Variables|Default|SetCalmMusic _returnvalue_2))
            (Audio|Components|Audio|Play _output_get_2 0.0)
            (Variables|Default|SetCalmMusicPlaying true)
            (Variables|Default|SetStressMusicPlaying false)))))))

(event EventBeginPlay
  (Variables|Default|SetCalmMusicPlaying true)
  (bind _returnvalue (Audio|CreateSound2D "/Game/Sounds_BPs/MS_MusicCalm_00.MS_MusicCalm_00" 1.0 1.0 0.0 0))
  (bind _output_get (Variables|Default|SetCalmMusic _returnvalue))
  (Audio|Components|Audio|Play _output_get 0.0)
  (bind _returnvalue_2 (Audio|CreateSound2D "/Game/Sounds_BPs/MS_MusicStress_00.MS_MusicStress_00" 1.0 1.0 0.0 0))
  (Variables|Default|SetStressMusic _returnvalue_2)
  (CallFunction|SpawnEnnemies)
  (Variables|Default|SetCurrentScore 0.0)
  (Variables|Default|SetCurrentMultiplier 1.0)
  (bind _returnvalue_3 (UserInterface|CreateWidget "/Game/Core/WB_Interface.WB_Interface_C"))
  (bind _output_get_2 (Variables|Default|SetHUDWidget _returnvalue_3))
  (UserInterface|Viewport|AddtoViewport _output_get_2 0)
  (Default|UpdateHUD _output_get_2))

(event EventTick
  (params (DeltaSeconds :type Float%20%28single-precision%29)))

(fn ConstructionScript)